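; Checkpoint actor that records a respawn location when something overlaps its zone.
; On begin overlap of ChechpointZone, it casts the game mode to Bp_GameMode and writes the zone's world location to LocationCheckpoint, without filtering the overlapping actor.
; Unconnected leftover nodes for calling Death and moving the player pawn to PlayerStart never run.
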(event `self.ChechpointZone.OnComponentBeginOverlap`
  (params (OverlappedComponent :type "PrimitiveComponent Object Reference") (OtherActor :type "Actor Object Reference") (OtherComp :type "PrimitiveComponent Object Reference") (OtherBodyIndex :type Integer) (bFromSweep :type Boolean) (SweepResult :type "HitResult Structure (by ref)"))
  (bind _asbp_game_mode (cast `/Game/Blueprints/Bp_GameMode` (`GameplayStatics.GetGameMode`)))
  (set `/Game/Blueprints/Bp_GameMode.LocationCheckpoint` (`SceneComponent.K2_GetComponentLocation` OverlappedComponent) _asbp_game_mode))

(fn `UserConstructionScript`)