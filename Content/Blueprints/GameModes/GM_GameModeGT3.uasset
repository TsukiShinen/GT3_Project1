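; Game mode that manages player life HUD, victory and defeat screens, checkpoint respawn and switching between playable characters.
; BeginPlay sets a default checkpoint and focus target and shows the Life widget; Victory pauses and shows its UI.
; Death shows the pause-and-defeat screen if the Perso roster is empty, otherwise removes the current character and possesses the first remaining with Niagara effect.
; SpawnCheckpoint resets Life and moves the player to the saved checkpoint.
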(event `self.ReceiveBeginPlay`
  ;[1 1 1] Initial Spawn
  (set `self.LocationCheckpoint` (3110.0 920.0 120.0))
  (set `self.FocusTarget` (`GameplayStatics.GetPlayerCharacter` 0))
  (bind _returnvalue (`|CreateWidget` "/Game/UI/Life.Life_C"))
  (`UserWidget.AddToViewport` _returnvalue 0))

(event `Victory`
  ;[1 1 1] Victory
  (`GameplayStatics.SetGamePaused` true)
  (set `PlayerController.bShowMouseCursor` true (`GameplayStatics.GetPlayerController` 0))
  (bind _returnvalue (`|CreateWidget` "/Game/UI/UI_Victory.UI_Victory_C"))
  (`UserWidget.AddToViewport` _returnvalue 0))

(event `Death`
  ;[1 1 1] Death
  (if (<= (`KismetArrayLibrary.Array_Length` (`self.Perso`)) 0)
    (`GameplayStatics.SetGamePaused` true)
    (set `PlayerController.bShowMouseCursor` true (`GameplayStatics.GetPlayerController` 0))
    (bind _returnvalue (`|CreateWidget` "/Game/UI/UI_Death.UI_Death_C"))
    (`UserWidget.AddToViewport` _returnvalue 0)
    (`KismetSystemLibrary.PrintString` "Hello")
    (else
      (`self.CharacterDieAndSwitch`))))

(event `SpawnCheckpoint`
  ;[1 1 1] Respawn
  (bind _asgm_game_mode_gt3 (cast `/Game/Blueprints/GameModes/GM_GameModeGT3` (`GameplayStatics.GetGameMode`)))
  (bind _locationcheckpoint (`/Game/Blueprints/GameModes/GM_GameModeGT3.LocationCheckpoint` _asgm_game_mode_gt3))
  (if (not (== (0.0 0.0 0.0) _locationcheckpoint))
    (bind _asbp_third_person_character (cast `/Game/ThirdPerson/Blueprints/BP_ThirdPersonCharacter` (`GameplayStatics.GetPlayerPawn` 0)))
    (set `/Game/ThirdPerson/Blueprints/BP_ThirdPersonCharacter.Life` 200.0 _asbp_third_person_character)
    (`self.K2_SetActorLocation` (`GameplayStatics.GetPlayerCharacter` 0) _locationcheckpoint false false)))

(fn `CharacterDieAndSwitch`
  (bind _perso (`self.Perso`))
  (`KismetArrayLibrary.Array_Remove` _perso (`self.currentPerso`))
  (bind _output_get (set `self.currentPerso` 0))
  (bind _output (`|GetArrayItem` _perso _output_get))
  (bind _aspawn (cast `Pawn` _output))
  (`Controller.Possess` (`GameplayStatics.GetPlayerController` 0) _aspawn)
  (`NiagaraFunctionLibrary.SpawnSystemAtLocation` "/Game/Materials/P_SwitchCharacter.P_SwitchCharacter" (`self.K2_GetActorLocation` _output)))

(fn `SwitchPawn`
  (params (Pawn :type "Pawn Object Reference"))
  (`Controller.Possess` (`GameplayStatics.GetPlayerController` 0) Pawn))

(fn `UserConstructionScript`)