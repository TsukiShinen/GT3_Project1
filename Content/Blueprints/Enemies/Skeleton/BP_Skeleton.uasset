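; Skeleton archer enemy that fires physics-driven arrows at the game mode's current focus target.
; BeginPlay caches the GM_GameModeGT3 reference, and BowMontage plays the draw animation on the separate Bow skeletal mesh.
; Shoot spawns BP_Arrow at the Arrow1 component, oriented toward FocusTarget, then launches its static mesh with an impulse along that direction.
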(event `self.ReceiveBeginPlay`
  (`parent.ReceiveBeginPlay`)
  (bind _asgm_game_mode_gt3 (cast `/Game/Blueprints/GameModes/GM_GameModeGT3` (`GameplayStatics.GetGameMode`)))
  (set `self.As GM Game Mode GT3` _asgm_game_mode_gt3))

(event `BowMontage`
  (`|PlayMontage` (`self.Bow`) "/Game/Blueprints/Enemies/Skeleton/AM_Bow.AM_Bow"))

(event `Shoot`
  (bind _returnvalue (`SceneComponent.K2_GetComponentLocation` (`self.Arrow1`)))
  (bind _returnvalue_2 (`KismetMathLibrary.GetDirectionUnitVector` _returnvalue (`self.K2_GetActorLocation` (`/Game/Blueprints/GameModes/GM_GameModeGT3.FocusTarget` (`self.As GM Game Mode GT3`)))))
  (bind _returnvalue_3 (`|SpawnActorFromClass` "/Game/Blueprints/Enemies/Skeleton/BP_Arrow.BP_Arrow_C" (`KismetMathLibrary.MakeTransform` _returnvalue (`KismetMathLibrary.Conv_VectorToRotator` _returnvalue_2)) "Undefined" "OverrideRootScale" null null))
  (`/Engine/EditorBlueprintResources/StandardMacros.IsValid` _returnvalue_3
    (:`Is Valid`
      (`PrimitiveComponent.AddImpulse` (`/Game/Blueprints/Enemies/BP_Projectile.StaticMesh` _returnvalue_3) (* _returnvalue_2 2000.0) "None" false))))

(fn `UserConstructionScript`
  (`parent.UserConstructionScript`))