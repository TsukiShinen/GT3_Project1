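; BP_Zombie is an enemy that deals periodic melee-range damage to actors entering its Box component.
; On BeginPlay it stores itself, cast to BP_Enemy, as a reference for filtering itself out of overlaps.
; An overlap sets an attack flag and starts a looping one-second timer that applies damage to the overlapped actor.
; No end-overlap logic clears the flag or timer.
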(event `self.ReceiveBeginPlay`
  (bind _asbp_enemy (cast `/Game/Blueprints/Enemies/BP_Enemy` self))
  (set `self.Enemy` _asbp_enemy)
  (`KismetSystemLibrary.PrintString` "ok"))

(event `self.Box.OnComponentBeginOverlap`
  (params (OverlappedComponent :type "PrimitiveComponent Object Reference") (OtherActor :type "Actor Object Reference") (OtherComp :type "PrimitiveComponent Object Reference") (OtherBodyIndex :type Integer) (bFromSweep :type Boolean) (SweepResult :type "HitResult Structure (by ref)"))
  (bind _returnvalue (!= OtherActor (`self.Enemy`)))
  (if _returnvalue
    (set `self.isAttack` _returnvalue)
    (`KismetSystemLibrary.K2_SetTimerDelegate` (delegate `AttackLoop`) 1.0 true)))

(event `AttackLoop`
  (if (`self.isAttack`)
    (`GameplayStatics.ApplyDamage` (stale `self.Box.OnComponentBeginOverlap` OtherActor) 10.0 null self)))

(fn `UserConstructionScript`)