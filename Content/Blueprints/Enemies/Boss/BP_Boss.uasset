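; Boss enemy Blueprint for the first phase of a boss fight, which swaps itself for BP_Boss2 at half health.
; Tick watches Life against BaseLife and, once below half, fires a one-time phase change.
; The change detaches the controller, spawns transition particles and an AI-controlled BP_Boss2 in place, passes on Life, BaseLife and Spawner, then destroys this actor.
; BeginPlay also caches the GM_GameModeGT3 game mode after a short delay.
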(event `self.ReceiveBeginPlay`
  (`parent.ReceiveBeginPlay`)
  (`KismetSystemLibrary.Delay` 0.2)
  (`|ExecutionSequence`
    (:`then_0`
      ;[1 1 1] Get GameMode
      (bind _asgm_game_mode_gt3 (cast `/Game/Blueprints/GameModes/GM_GameModeGT3` (`GameplayStatics.GetGameMode`)))
      (set `self.Game Mode GT3` _asgm_game_mode_gt3))))

(event `self.ReceiveTick`
  (params (DeltaSeconds :type "Float (single-precision)"))
  (bind (_returnvalue_location _returnvalue_rotation) (`KismetMathLibrary.BreakTransform` (`SceneComponent.K2_GetComponentToWorld` (`self.CapsuleComponent`))))
  (`parent.ReceiveTick` DeltaSeconds)
  (`|ExecutionSequence`
    (:`then_0`
      ;[1 1 1] Get IsUnderMidHp
      (if (< (`self.Life`) (/ (`self.Base Life`) 2.0))
        (set `self.IsUnderMidHp` true)))
    (:`then_1`
      ;[1 1 1] Change Phase
      (if (`self.IsUnderMidHp`)
        (`/Engine/EditorBlueprintResources/StandardMacros.DoOnce` false
          (:`Completed`
            (`self.DetachFromControllerPendingDestroy`)
            (`|SpawnActorFromClass` "/Game/Blueprints/Enemies/Boss/BP_ChangePhaseParticles.BP_ChangePhaseParticles_C" (`SceneComponent.K2_GetComponentToWorld` (`self.CapsuleComponent`)) "Undefined" "OverrideRootScale" null null)
            (`PrimitiveComponent.SetCollisionEnabled` (`self.Cylinder`) "NoCollision")
            (bind _returnvalue (`AIBlueprintHelperLibrary.SpawnAIFromClass` "/Game/Blueprints/Enemies/Boss/BP_Boss2.BP_Boss2_C" null _returnvalue_location _returnvalue_rotation false null))
            (bind _asbp_boss_2 (cast `/Game/Blueprints/Enemies/Boss/BP_Boss2` _returnvalue))
            (set `/Game/Blueprints/Enemies/BP_Enemy.Life` (`self.Life`) _asbp_boss_2)
            (set `/Game/Blueprints/Enemies/BP_Enemy.Base Life` (`self.Base Life`) _asbp_boss_2)
            (set `/Game/Blueprints/Enemies/Boss/BP_Boss.Spawner` (`self.Spawner`) _asbp_boss_2)
            (`self.K2_DestroyActor`)))))))

(fn `UserConstructionScript`
  (`parent.UserConstructionScript`))