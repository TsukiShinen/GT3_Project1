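; BP_Boss2 is a boss enemy Blueprint that triggers victory when it dies.
; It runs the parent's BeginPlay and construction script, then each Tick orients its health bar and checks Life.
; At zero or below, it prints a debug "Hello" and calls Victory on GameModeGT30, with no guard against repeating on later frames.
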(event `self.ReceiveBeginPlay`
  (`parent.ReceiveBeginPlay`))

(event `self.ReceiveTick`
  (params (DeltaSeconds :type "Float (single-precision)"))
  (`|ExecutionSequence`
    (:`then_0`
      (`self.Health Bar Look At`))
    (:`then_1`
      (if (<= (`self.Life`) 0.0)
        (`KismetSystemLibrary.PrintString` "Hello")
        (`/Game/Blueprints/GameModes/GM_GameModeGT3.Victory` (`self.Game Mode GT3_0`))))))

(fn `UserConstructionScript`
  (`parent.UserConstructionScript`))