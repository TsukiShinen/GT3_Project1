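; BP_Spawner is a one-shot enemy spawner that fires the first time anything overlaps its Range component.
; A ForLoopDelay macro, a for loop with a Delay between iterations, spawns NbrEntity AI pawns of the Entity class at the spawner's transform, spaced by TimeBetweenSpawn.
; The spawner destroys itself once the loop completes.
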(event `self.Range.OnComponentBeginOverlap`
  (params (OverlappedComponent :type "PrimitiveComponent Object Reference") (OtherActor :type "Actor Object Reference") (OtherComp :type "PrimitiveComponent Object Reference") (OtherBodyIndex :type Integer) (bFromSweep :type Boolean) (SweepResult :type "HitResult Structure (by ref)"))
  (bind (_returnvalue_location _returnvalue_rotation) (`KismetMathLibrary.BreakTransform` (`self.GetTransform`)))
  (`/Engine/EditorBlueprintResources/StandardMacros.DoOnce` false
    (:`Completed`
      (`self.ForLoopDelay` 1 (`self.NbrEntity`) (`self.TimeBetweenSpawn`)
        (:`Body`
          (`AIBlueprintHelperLibrary.SpawnAIFromClass` (`self.Entity`) null _returnvalue_location _returnvalue_rotation false null))
        (:`Completed`
          (`self.K2_DestroyActor`))))))

(fn `UserConstructionScript`)