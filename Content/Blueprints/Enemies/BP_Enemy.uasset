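; BP_Enemy is an enemy actor that tracks its own Life, starting from BaseLife, and is destroyed when it runs out.
; AnyDamage reduces Life only when the damage causer is the player pawn or BP_Companion, then checks for death.
; Tick refreshes a TextRender with the current Life every frame and repeats the death check.
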(event `self.ReceiveBeginPlay`
  ;[1 1 1] Init
  (set `self.Life` (`self.Base Life`)))

(event `self.ReceiveTick`
  (params (DeltaSeconds :type "Float (single-precision)"))
  (`|ExecutionSequence`
    (:`then_0`
      ;[1 1 1] Set Life Display
      (`TextRenderComponent.K2_SetText` (`self.TextRender`) (`KismetTextLibrary.Conv_DoubleToText` (`self.Life`) "HalfToEven")))
    (:`then_1`
      ;[1 1 1] Is dead ?
      (if (<= (`self.Life`) 0.0)
        (`self.K2_DestroyActor`)))))

(event `self.ReceiveAnyDamage`
  (params (Damage :type "Float (single-precision)") (DamageType :type "DamageType Object Reference") (InstigatedBy :type "Controller Object Reference") (DamageCauser :type "Actor Object Reference"))
  ;[1 1 1] Any Damage
  (if (or (== (`GameplayStatics.GetPlayerPawn` 0) DamageCauser) (== DamageCauser "/Game/Blueprints/Characters/Wirael/BP_Companion.BP_Companion"))
    (bind _output_get (set `self.Life` (- (`self.Life`) Damage)))
    (if (<= _output_get 0.0)
      (`self.K2_DestroyActor`))))

(fn `UserConstructionScript`)