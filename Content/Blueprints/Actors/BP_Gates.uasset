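; Arena gate actor that blocks the exits when its trigger box is entered and reopens them when the challenge is completed.
; Box overlap, with no check on the overlapping actor, unhides the walls and enables their collision; OnChallengeCompleted hides them and disables it.
; Both events find the walls by scanning every StaticMeshActor in the level for the display name "WallBlockTrigger", rather than holding references.
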(event `self.Box.OnComponentBeginOverlap`
  (params (OverlappedComponent :type "PrimitiveComponent Object Reference") (OtherActor :type "Actor Object Reference") (OtherComp :type "PrimitiveComponent Object Reference") (OtherBodyIndex :type Integer) (bFromSweep :type Boolean) (SweepResult :type "HitResult Structure (by ref)"))
  ;[1 1 1] Ferme les portes d'une arène lorsqu'on y rentre (avec une trigger box)
  (bind _outactors (`GameplayStatics.GetAllActorsOfClass` "/Script/Engine.StaticMeshActor"))
  (for _array_element _outactors
    (if (`KismetStringLibrary.EqualEqual_StrStr` "WallBlockTrigger" (`KismetSystemLibrary.GetDisplayName` _array_element))
      (`self.SetActorHiddenInGame` _array_element false)
      (`PrimitiveComponent.SetCollisionEnabled` (`StaticMeshActor.StaticMeshComponent` _array_element) "QueryAndPhysics"))))

(event `OnChallengeCompleted`
  ;[1 1 1] Ouvre les portes d'une arène lorsqu'on y rentre
  (bind _outactors (`GameplayStatics.GetAllActorsOfClass` "/Script/Engine.StaticMeshActor"))
  (for _array_element _outactors
    (if (`KismetStringLibrary.EqualEqual_StrStr` "WallBlockTrigger" (`KismetSystemLibrary.GetDisplayName` _array_element))
      (`self.SetActorHiddenInGame` _array_element true)
      (`PrimitiveComponent.SetCollisionEnabled` (`StaticMeshActor.StaticMeshComponent` _array_element) "NoCollision"))))

(fn `UserConstructionScript`)