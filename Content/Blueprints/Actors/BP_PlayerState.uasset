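; BP_PlayerState tracks the player's Life and Alive state, with an M key binding that drains life.
; Each M press subtracts a fixed amount from Life and prints the result while Life is nonzero.
; Pressing M at zero Life instead calls Die on BP_PlayerController.
; Tick separately polls Life and clears Alive when it equals exactly zero.
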(event `self.ReceiveBeginPlay`)

(event `Key|M`
  (params (Key :type "Key Structure"))
  (:`Pressed`
    (if (== 0 (`self.Life`))
      (bind _asbp_player_controller (cast `/Game/Blueprints/Characters/BP_PlayerController` (`GameplayStatics.GetPlayerController` 0)))
      (`/Game/Blueprints/Characters/BP_PlayerController.Die` _asbp_player_controller)
      (else
        (bind _output_get (set `self.Life` (- (`self.Life`) 2)))
        (`KismetSystemLibrary.PrintString` (`KismetStringLibrary.Conv_IntToString` _output_get))))))

(event `self.ReceiveTick`
  (params (DeltaSeconds :type "Float (single-precision)"))
  (if (== (`self.Life`) 0)
    (set `self.Alive` false)))

(fn `UserConstructionScript`)