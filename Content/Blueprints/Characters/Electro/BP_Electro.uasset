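; Electro player character with three skills: electric arc, projectile counter and dash.
; Holding Skill 1 spawns an arc actor, stretched each Tick from the player to a screen-center line trace.
; Holding Skill 2 enables a collider that redirects pumpkin projectiles toward the crosshair, claiming damage credit only when that trace hits.
; Skill 3 hops then launches forward if hardcoded ZQSD keys are held, with a DoOnce-and-delay cooldown.
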(event `InputAction|Skill 1`
  (params (Key :type "Key Structure"))
  ;[1 1 1] Shoot electric arc
  (:`Pressed`
    (bind _returnvalue (`|SpawnActorFromClass` "/Game/Blueprints/Characters/Electro/BP_ElecticalArc.BP_ElecticalArc_C" (`self.GetTransform` (`GameplayStatics.GetPlayerPawn` 0)) "Undefined" "OverrideRootScale" null null))
    (set `self.ElectricArc` _returnvalue))
  (:`Released`
    (`self.K2_DestroyActor` (`self.ElectricArc`))
    (set `self.ElectricArc` null)))

(event `self.ReceiveTick`
  (params (DeltaSeconds :type "Float (single-precision)"))
  (bind _returnvalue (`GameplayStatics.GetPlayerPawn` 0))
  (bind _electricarc (`self.ElectricArc`))
  (bind _returnvalue_location (`KismetMathLibrary.BreakTransform` (`self.GetTransform` _returnvalue)))
  (bind (_returnvalue_x _returnvalue_y) (`KismetMathLibrary.BreakVector2D` (/ (`WidgetLayoutLibrary.GetViewportSize`) (2.0 2.0))))
  (bind (_worldlocation _worlddirection) (`PlayerController.DeprojectScreenPositionToWorld` (`PlayerState.GetPlayerController` (`Pawn.PlayerState` _returnvalue)) _returnvalue_x _returnvalue_y))
  ;[1 1 1] Shoot electric arc
  (`/Engine/EditorBlueprintResources/StandardMacros.IsValid` _electricarc
    (:`Is Valid`
      (`/Game/Blueprints/Characters/Electro/BP_ElecticalArc.SetStartPosition` _electricarc (`KismetMathLibrary.MakeTransform` _returnvalue_location))
      (bind (_outhit _returnvalue_2) (`KismetSystemLibrary.LineTraceSingle` _returnvalue_location (+ _worldlocation (* _worlddirection (`self.LaserRange`))) "TraceTypeQuery1"))
      (if _returnvalue_2
        (bind (_bblockinghit _binitialoverlap _time _distance _location _impactpoint _normal _impactnormal _physmat _hitactor _hitcomponent _hitbonename _bonename _hititem _elementindex _faceindex _tracestart _traceend) (`GameplayStatics.BreakHitResult` _outhit))
        (`/Game/Blueprints/Characters/Electro/BP_ElecticalArc.SetEndPosition` _electricarc (`KismetMathLibrary.MakeTransform` _impactpoint))
        (else
          (`/Game/Blueprints/Characters/Electro/BP_ElecticalArc.SetEndPosition` _electricarc (`KismetMathLibrary.MakeTransform` _traceend)))))))

(event `InputAction|Skill 3`
  (params (Key :type "Key Structure"))
  ;[1 1 1] Dash
  (:`Pressed`
    (bind _returnvalue (`self.GetMovingInput`))
    (if _returnvalue
      (`/Engine/EditorBlueprintResources/StandardMacros.DoOnce` false :!label _label
        (:`Completed`
          (`self.LaunchCharacter` (0.0 0.0 200.0))
          (`KismetSystemLibrary.Delay` 0.1)
          (`self.LaunchCharacter` (* (`self.GetActorForwardVector`) 1000.0))
          (`KismetSystemLibrary.Delay` 1.0)
          (goto _label :!via `Reset`))))))

(event `self.ReceiveBeginPlay`
  ;[1 1 1] Counter
  (`PrimitiveComponent.SetCollisionEnabled` (`self.ProjectileCounter`) "NoCollision" :!label _label_2))

(event `InputAction|Skill 2`
  (params (Key :type "Key Structure"))
  ;[1 1 1] Counter
  (:`Pressed`
    (`PrimitiveComponent.SetCollisionEnabled` (`self.ProjectileCounter`) "QueryAndPhysics"))
  (:`Released`
    (goto _label_2)))

(event `self.ProjectileCounter.OnComponentBeginOverlap`
  (params (OverlappedComponent :type "PrimitiveComponent Object Reference") (OtherActor :type "Actor Object Reference") (OtherComp :type "PrimitiveComponent Object Reference") (OtherBodyIndex :type Integer) (bFromSweep :type Boolean) (SweepResult :type "HitResult Structure (by ref)"))
  (bind (_returnvalue_x _returnvalue_y) (`KismetMathLibrary.BreakVector2D` (/ (`WidgetLayoutLibrary.GetViewportSize`) (2.0 2.0))))
  (bind (_worldlocation _worlddirection) (`PlayerController.DeprojectScreenPositionToWorld` (`GameplayStatics.GetPlayerController` 0) _returnvalue_x _returnvalue_y))
  (bind _returnvalue (+ _worldlocation (* _worlddirection 10000.0)))
  ;[1 1 1] Counter
  (bind _asbp_pumpkin_projectile (cast `/Game/Blueprints/Enemies/Pumpkin/BP_PumpkinProjectile` OtherActor))
  (bind _staticmesh (`/Game/Blueprints/Enemies/Pumpkin/BP_PumpkinProjectile.StaticMesh` _asbp_pumpkin_projectile))
  (`PrimitiveComponent.SetPhysicsLinearVelocity` _staticmesh (0.0 0.0 0.0) false "None")
  (bind _returnvalue_2 (`SceneComponent.K2_GetComponentLocation` _staticmesh))
  (bind (_outhit _returnvalue_3) (`KismetSystemLibrary.LineTraceSingle` _returnvalue_2 _returnvalue "TraceTypeQuery1"))
  (if _returnvalue_3
    (`PrimitiveComponent.AddImpulse` _staticmesh (* (`KismetMathLibrary.GetDirectionUnitVector` _returnvalue_2 (`.ImpactPoint` (`GameplayStatics.BreakHitResult` _outhit))) 1500.0) "None" false)
    (set `/Game/Blueprints/Enemies/Pumpkin/BP_PumpkinProjectile.DamageDealer` self _asbp_pumpkin_projectile)
    (else
      (`PrimitiveComponent.AddImpulse` _staticmesh (* (`KismetMathLibrary.GetDirectionUnitVector` _returnvalue_2 _returnvalue) 1500.0) "None" false))))

(fn `GetMovingInput`
  (returns (ReturnValue :type Boolean))
  (bind _returnvalue (`GameplayStatics.GetPlayerController` 0))
  (return (or (`PlayerController.IsInputKeyDown` _returnvalue "Z") (`PlayerController.IsInputKeyDown` _returnvalue "S") (`PlayerController.IsInputKeyDown` _returnvalue "Q") (`PlayerController.IsInputKeyDown` _returnvalue "D"))))

(fn `UserConstructionScript`)