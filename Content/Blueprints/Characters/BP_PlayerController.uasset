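; Player controller that lets the player switch between three characters: Sven, Wirael and Electro.
; BeginPlay spawns all three at the player pawn's transform and possesses Sven, leaving the others in their unpossessed state.
; Switch inputs call PossessCharacter, which moves the target onto the current character's location and rotation before possessing it.
; Short delays then restore the saved control rotation and run the new character's post-possess update.
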(event `self.ReceiveBeginPlay`
  (bind _returnvalue (`self.GetTransform` (`GameplayStatics.GetPlayerPawn` 0)))
  (bind _returnvalue_2 (`|SpawnActorFromClass` "/Game/Blueprints/Characters/Sven/BP_Sven.BP_Sven_C" _returnvalue "Undefined" "OverrideRootScale" null null))
  (bind _output_get (set `self.BP Sven` _returnvalue_2))
  (`self.Possess` (`GameplayStatics.GetPlayerController` 0) _output_get)
  (`/Game/ThirdPerson/Blueprints/BP_ThirdPersonCharacter.UpdateCharacterAfterPossess` _output_get)
  (set `self.CurrentCharatere` _returnvalue_2)
  (bind _returnvalue_3 (`|SpawnActorFromClass` "/Game/Blueprints/Characters/Wirael/BP_Wirael.BP_Wirael_C" _returnvalue "Undefined" "OverrideRootScale" null null))
  (bind _output_get_2 (set `self.BP_Wirael` _returnvalue_3))
  (`/Game/ThirdPerson/Blueprints/BP_ThirdPersonCharacter.UpdateCharacterBeforeUnpossess` _output_get_2)
  (bind _returnvalue_4 (`|SpawnActorFromClass` "/Game/Blueprints/Characters/Electro/BP_Electro.BP_Electro_C" _returnvalue "Undefined" "OverrideRootScale" null null))
  (bind _output_get_3 (set `self.BP_Electro` _returnvalue_4))
  (`/Game/ThirdPerson/Blueprints/BP_ThirdPersonCharacter.UpdateCharacterBeforeUnpossess` _output_get_3))

(event `InputAction|SwitchSven`
  (params (Key :type "Key Structure"))
  (bind _bp_sven (`self.BP Sven`))
  (:`Pressed`
    (`self.Possess Character` _bp_sven)
    (`KismetSystemLibrary.Delay` 0.05)
    (`self.SetControlRotation` (`GameplayStatics.GetPlayerController` 0) (`self.Previous controller rotation`))
    (bind _output_get (set `self.CurrentCharatere` _bp_sven))
    (`KismetSystemLibrary.Delay` 0.05)
    (`/Game/ThirdPerson/Blueprints/BP_ThirdPersonCharacter.UpdateCharacterAfterPossess` _output_get)))

(event `InputAction|SwitchWirael`
  (params (Key :type "Key Structure"))
  (bind _bp_wirael (`self.BP_Wirael`))
  (:`Pressed`
    (`self.Possess Character` _bp_wirael)
    (`KismetSystemLibrary.Delay` 0.05)
    (`self.SetControlRotation` (`GameplayStatics.GetPlayerController` 0) (`self.Previous controller rotation`))
    (bind _output_get (set `self.CurrentCharatere` _bp_wirael))
    (`KismetSystemLibrary.Delay` 0.05)
    (`/Game/ThirdPerson/Blueprints/BP_ThirdPersonCharacter.UpdateCharacterAfterPossess` _output_get)))

(event `InputAction|SwitchElectro`
  (params (Key :type "Key Structure"))
  (bind _bp_electro (`self.BP_Electro`))
  (:`Pressed`
    (`self.Possess Character` _bp_electro)
    (`KismetSystemLibrary.Delay` 0.05)
    (`self.SetControlRotation` (`GameplayStatics.GetPlayerController` 0) (`self.Previous controller rotation`))
    (bind _output_get (set `self.CurrentCharatere` _bp_electro))
    (`KismetSystemLibrary.Delay` 0.05)
    (`/Game/ThirdPerson/Blueprints/BP_ThirdPersonCharacter.UpdateCharacterAfterPossess` _output_get)))

(fn `Possess Character`
  (params (To :type "/Game/ThirdPerson/Blueprints/BP_ThirdPersonCharacter Object Reference"))
  (bind _currentcharatere (`self.CurrentCharatere`))
  (if (!= To (`GameplayStatics.GetObjectClass` _currentcharatere))
    (`/Game/ThirdPerson/Blueprints/BP_ThirdPersonCharacter.UpdateCharacterBeforeUnpossess` _currentcharatere)
    (set `self.Previous controller rotation` (`self.GetControlRotation`))
    (`self.K2_SetActorLocationAndRotation` To (`self.K2_GetActorLocation` _currentcharatere) (`self.K2_GetActorRotation` _currentcharatere) false false)
    (`self.Possess` (`GameplayStatics.GetPlayerController` 0) To)))

(fn `UserConstructionScript`)