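; BP_BasicPotion is a potion flask that deals area damage and explodes on impact.
; When the flask mesh hits anything other than the player pawn, it stores the impact point, applies full radial damage there that spares the player, and destroys itself.
; The Destroyed event spawns BP_Explosion at the stored point, so any destruction of the actor triggers the explosion, not just a hit.
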(event `self.ReceiveDestroyed`
  (`|SpawnActorFromClass` "/Game/Blueprints/Characters/Sven/BP_Explosion.BP_Explosion_C" (`KismetMathLibrary.Conv_VectorToTransform` (`self.Impact Point`)) "Undefined" "OverrideRootScale" null null))

(event `self.S_Flask.OnComponentHit`
  (params (HitComponent :type "PrimitiveComponent Object Reference") (OtherActor :type "Actor Object Reference") (OtherComp :type "PrimitiveComponent Object Reference") (NormalImpulse :type "Vector Structure") (Hit :type "HitResult Structure (by ref)"))
  (bind _returnvalue (`GameplayStatics.GetPlayerPawn` 0))
  (if (!= OtherActor _returnvalue)
    (bind _output_get (set `self.Impact Point` (`.ImpactPoint` (`GameplayStatics.BreakHitResult` Hit))))
    (`GameplayStatics.ApplyRadialDamage` 50.0 _output_get 200.0 null (`|MakeArray` _returnvalue :!type "Actor Object Reference") _returnvalue null true)
    (`self.K2_DestroyActor`)))

(fn `UserConstructionScript`)