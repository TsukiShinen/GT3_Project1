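; BP_Sven is the Blueprint for Sven, a playable potion-thrower with basic, jump and heal attacks.
; Each skill input clears the CanAttack gate and plays a montage, whose notify states call back to spawn the potion or heal actor at a socket.
; Thrown flasks get a forward impulse (basic adds player velocity) while hiding the hand-held mesh, which reload events show again.
; CanAttack is not re-enabled in this graph.
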(event `ReloadLeftPotion`
  ;[1 1 1] Reload Potions
  (`SceneComponent.SetVisibility` (`self.S_Flask_L`) true false))

(event `self.ReceiveBeginPlay`
  ;[1 1 1] Get ABP_Sven
  (bind _asabp_sven (cast `/Game/Blueprints/Characters/Sven/ABP_Sven` (`SkeletalMeshComponent.GetAnimInstance` (`self.Mesh`))))
  (set `self.ABP Sven` _asabp_sven))

(event `ReloadRightPotion`
  ;[1 1 1] Reload Potions
  (`SceneComponent.SetVisibility` (`self.S_Flask_R`) true false))

(event `ThrowBasicAttack`
  (bind _leftsocket (`self.LeftSocket`))
  ;[1 1 1] Throw Basic Attack (Called in BP_BasicAttacking (notify state))
  (`SceneComponent.SetVisibility` (`self.S_Flask_L`) false false)
  (bind _returnvalue (`|SpawnActorFromClass` "/Game/Blueprints/Characters/Sven/BP_BasicPotion.BP_BasicPotion_C" (`SceneComponent.K2_GetComponentToWorld` _leftsocket) "Undefined" "OverrideRootScale" null null))
  (`PrimitiveComponent.AddImpulse` (`/Game/Blueprints/Characters/Sven/BP_BasicPotion.S_Flask` _returnvalue) (+ (* (`SceneComponent.GetForwardVector` _leftsocket) (`self.ThrowForce`)) (`CharacterMovementComponent.GetLastUpdateVelocity` (`Character.CharacterMovement` (`GameplayStatics.GetPlayerCharacter` 0)))) "None" false))

(event `InputAction|Skill 1`
  (params (Key :type "Key Structure"))
  ;[1 1 1] Basic Attack
  (:`Pressed`
    (if (`self.canAttack`)
      (set `self.canAttack` false)
      (`|PlayMontage` (`self.Mesh`) "/Game/Third_Party/UndeadPack/EnemyGoblin/Animations/Anim_Attack2_Montage.Anim_Attack2_Montage"))))

(event `InputAction|Skill 2`
  (params (Key :type "Key Structure"))
  ;[1 1 1] Jump Attack
  (:`Pressed`
    (if (`self.canAttack`)
      (set `self.canAttack` false)
      (`|PlayMontage` (`self.Mesh`) "/Game/Third_Party/UndeadPack/EnemyGoblin/Animations/Anim_Attack1_Montage.Anim_Attack1_Montage"))))

(event `ThrowJumpAttack`
  (bind _rightsocket (`self.RightSocket`))
  ;[1 1 1] Throw Jump Attack (Called in BP_JumpAttacking (notify state))
  (`SceneComponent.SetVisibility` (`self.S_Flask_R`) false false)
  (bind _returnvalue (`|SpawnActorFromClass` "/Game/Blueprints/Characters/Sven/BP_JumpPotion.BP_JumpPotion_C" (`SceneComponent.K2_GetComponentToWorld` _rightsocket) "Undefined" "OverrideRootScale" null null))
  (`PrimitiveComponent.AddImpulse` (`/Game/Blueprints/Characters/Sven/BP_JumpPotion.S_Flask` _returnvalue) (* (`SceneComponent.GetForwardVector` _rightsocket) (`self.ThrowForce`)) "None" false))

(event `ThrowHealAttack`
  ;[1 1 1] ThrowHealAttack (Called in BP_HealAttacking (notify state))
  (`|SpawnActorFromClass` "/Game/Blueprints/Characters/Sven/BP_Heal.BP_Heal_C" (`SceneComponent.K2_GetComponentToWorld` (`self.HealSocket`)) "Undefined" "OverrideRootScale" null null))

(event `InputAction|Skill 3`
  (params (Key :type "Key Structure"))
  ;[1 1 1] Heal Attack
  (:`Pressed`
    (if (`self.canAttack`)
      (set `self.canAttack` false)
      (`|PlayMontage` (`self.Mesh`) "/Game/Third_Party/UndeadPack/EnemyGoblin/Animations/Anim_Agr_Montage.Anim_Agr_Montage"))))

(fn `UserConstructionScript`)