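; BP_JumpPotion is a potion flask that leaves a jump boost and an explosion where it lands.
; A hit on S_Flask stores the impact point and destroys the actor, guarded by a check comparing the hit component, rather than its actor, to the player pawn.
; The Destroyed event then spawns BP_JumpBoost and BP_Explosion at the stored point.
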(event `self.ReceiveDestroyed`
  (bind _returnvalue (`KismetMathLibrary.Conv_VectorToTransform` (`self.Impact Point`)))
  (`|SpawnActorFromClass` "/Game/Blueprints/Characters/Sven/BP_JumpBoost.BP_JumpBoost_C" _returnvalue "Undefined" "OverrideRootScale" null null)
  (`|SpawnActorFromClass` "/Game/Blueprints/Characters/Sven/BP_Explosion.BP_Explosion_C" _returnvalue "Undefined" "OverrideRootScale" null null))

(event `self.S_Flask.OnComponentHit`
  (params (HitComponent :type "PrimitiveComponent Object Reference") (OtherActor :type "Actor Object Reference") (OtherComp :type "PrimitiveComponent Object Reference") (NormalImpulse :type "Vector Structure") (Hit :type "HitResult Structure (by ref)"))
  (if (!= OtherComp (`GameplayStatics.GetPlayerPawn` 0))
    (set `self.Impact Point` (`.ImpactPoint` (`GameplayStatics.BreakHitResult` Hit)))
    (`self.K2_DestroyActor`)))

(fn `UserConstructionScript`)