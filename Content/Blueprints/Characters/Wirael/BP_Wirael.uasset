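; BP_Wirael is the Wirael character, with an area attack and an AI companion called Cactus.
; Skill 1 damages every enemy tracked by the overlap box.
; Skill 3 spawns Cactus once, or sends a living one outside attack mode to a screen-center line trace hit, with debug drawing left on.
; Skill 2 flip-flops Cactus's attack mode, and ResetCactus re-arms the spawn after a short delay.
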(event `self.Box.OnComponentBeginOverlap`
  (params (OverlappedComponent :type "PrimitiveComponent Object Reference") (OtherActor :type "Actor Object Reference") (OtherComp :type "PrimitiveComponent Object Reference") (OtherBodyIndex :type Integer) (bFromSweep :type Boolean) (SweepResult :type "HitResult Structure (by ref)"))
  (bind _asbp_enemy (cast `/Game/Blueprints/Enemies/BP_Enemy` OtherActor))
  (`KismetArrayLibrary.Array_AddUnique` (`self.ListOfEnemyCanAttack`) _asbp_enemy))

(event `self.Box.OnComponentEndOverlap`
  (params (OverlappedComponent :type "PrimitiveComponent Object Reference") (OtherActor :type "Actor Object Reference") (OtherComp :type "PrimitiveComponent Object Reference") (OtherBodyIndex :type Integer))
  (bind _asbp_enemy (cast `/Game/Blueprints/Enemies/BP_Enemy` OtherActor))
  (`KismetArrayLibrary.Array_RemoveItem` (`self.ListOfEnemyCanAttack`) _asbp_enemy))

(event `InputAction|Skill 1`
  (params (Key :type "Key Structure"))
  (:`Pressed`
    (for _array_element (`self.ListOfEnemyCanAttack`)
      (`GameplayStatics.ApplyDamage` _array_element 2.0 null self))))

(event `InputAction|Skill 3`
  (params (Key :type "Key Structure"))
  (bind _returnvalue (`GameplayStatics.GetPlayerPawn` 0))
  (bind _cactus (`self.Cactus`))
  (bind _returnvalue_location (`KismetMathLibrary.BreakTransform` (`self.GetTransform` _returnvalue)))
  (bind _returnvalue_location_2 (`KismetMathLibrary.BreakTransform` (`SceneComponent.K2_GetComponentToWorld` (`self.Mesh`))))
  (bind (_returnvalue_x _returnvalue_y) (`KismetMathLibrary.BreakVector2D` (/ (`WidgetLayoutLibrary.GetViewportSize`) (2.0 2.0))))
  (bind (_worldlocation _worlddirection) (`PlayerController.DeprojectScreenPositionToWorld` (`PlayerState.GetPlayerController` (`Pawn.PlayerState` _returnvalue)) _returnvalue_x _returnvalue_y))
  (:`Pressed`
    (`/Engine/EditorBlueprintResources/StandardMacros.IsValid` _cactus
      (:`Is Valid`
        (if (not (`/Game/Blueprints/Characters/Wirael/BP_Companion.isAttackMode` _cactus))
          (bind _outhit (`KismetSystemLibrary.LineTraceSingle` :`Start` _returnvalue_location :`End` (+ _worldlocation (* _worlddirection 50000.0)) :`TraceChannel` "TraceTypeQuery1" :`DrawDebugType` "ForDuration" :`DrawTime` 10.0))
          (set `/Game/Blueprints/Characters/Wirael/BP_Companion.LocationTarget` (`.Location` (`GameplayStatics.BreakHitResult` _outhit)) (`self.Cactus`))))
      (:`Is Not Valid`
        (`/Engine/EditorBlueprintResources/StandardMacros.DoOnce` false :!label _label
          (:`Completed`
            (bind _returnvalue_2 (`AIBlueprintHelperLibrary.SpawnAIFromClass` "/Game/Blueprints/Characters/Wirael/BP_Companion.BP_Companion_C" null (+ _returnvalue_location_2 (0.0 50.0 0.0)) (struct) false null))
            (bind _asbp_companion (cast `/Game/Blueprints/Characters/Wirael/BP_Companion` _returnvalue_2))
            (bind _output_get (set `self.Cactus` _asbp_companion))
            (set `/Game/Blueprints/Characters/Wirael/BP_Companion.Wirael` self _output_get)))))))

(event `InputAction|Skill 2`
  (params (Key :type "Key Structure"))
  (bind _cactus (`self.Cactus`))
  (:`Pressed`
    (`/Engine/EditorBlueprintResources/StandardMacros.FlipFlop`
      (:`A`
        (set `/Game/Blueprints/Characters/Wirael/BP_Companion.isAttackMode` false _cactus)
        (set `/Game/Blueprints/Characters/Wirael/BP_Companion.LocationTarget` (0.0 0.0 0.0) (`self.Cactus`)))
      (:`B`
        (set `/Game/Blueprints/Characters/Wirael/BP_Companion.isAttackMode` true _cactus)))
    (set `/Game/Blueprints/Characters/Wirael/BP_Companion.isTargeting` false _cactus)))

(event `Reset Cactus`
  (`KismetSystemLibrary.Delay` 3.0)
  (goto _label :!via `Reset`))

(fn `UserConstructionScript`)