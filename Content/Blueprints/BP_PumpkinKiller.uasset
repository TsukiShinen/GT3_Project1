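; BP_PumpkinKiller is an enemy turret that fires pumpkin projectiles at the player.
; Every tick it rotates its static mesh to face player character 0.
; A looping timer, set on BeginPlay from the shoot cooldown, makes the mesh hop with an upward physics impulse.
; After a short delay, it spawns a BP_PumpkinProjectile ahead of the mesh and launches it forward with an impulse.
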(event `self.ReceiveTick`
  (params (DeltaSeconds :type "Float (single-precision)"))
  ;[1 1 1] Look at player
  (`SceneComponent.K2_SetWorldRotation` (`self.StaticMesh`) (`KismetMathLibrary.Conv_VectorToRotator` (`KismetMathLibrary.GetDirectionUnitVector` (`SceneComponent.K2_GetComponentLocation` (`self.StaticMesh`)) (`self.K2_GetActorLocation` (`GameplayStatics.GetPlayerCharacter` 0)))) false false))

(event `self.ReceiveBeginPlay`
  (`KismetSystemLibrary.K2_SetTimerDelegate` (delegate `Shoot`) (`self.ShootCooldown`) true))

(event `Shoot`
  (bind _staticmesh (`self.StaticMesh`))
  (bind (_returnvalue_location _returnvalue_rotation _returnvalue_scale) (`KismetMathLibrary.BreakTransform` (`SceneComponent.K2_GetComponentToWorld` _staticmesh)))
  (bind _returnvalue (`SceneComponent.GetForwardVector` _staticmesh))
  (`PrimitiveComponent.AddImpulse` _staticmesh (0.0 0.0 500.0) "None" false)
  (`KismetSystemLibrary.Delay` 0.2)
  (bind _returnvalue_2 (`|SpawnActorFromClass` "/Game/Blueprints/BP_PumpkinProjectile.BP_PumpkinProjectile_C" (`KismetMathLibrary.MakeTransform` (+ _returnvalue_location (* _returnvalue 100.0)) _returnvalue_rotation _returnvalue_scale) "Undefined" "OverrideRootScale" null null))
  (`PrimitiveComponent.AddImpulse` (`/Game/Blueprints/BP_PumpkinProjectile.StaticMesh` _returnvalue_2) (* _returnvalue 1500.0) "None" false))

(fn `UserConstructionScript`)